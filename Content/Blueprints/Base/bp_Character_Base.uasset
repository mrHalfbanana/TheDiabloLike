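; Base character Blueprint that handles incoming damage and equips a weapon and skills.
; DoDamage passes damage amounts, types and dealer to CalculateDamage and subtracts the result from ActualHealth.
; SpawnWeaponAndSkills reads classes from player controller 0, spawns the weapon onto the mesh's RH socket, and fills the R, F, Q and C skill arrays with spawned actors.
; Temporary T and Y keys raise or lower the clamped School value.
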(event `/Game/Blueprints/Gameplay/Damage/i_Damagable.DoDamage`
  (params (InDamage :type "Float (single-precision)") (InDamageAdditional :type "Array of Float (single-precision) (by ref)") (InDamageType :type "/Game/Blueprints/Gameplay/Damage/e_DamageTypes Enum" :default "NewEnumerator0") (InDamageTypeAdditional :type "Array of /Game/Blueprints/Gameplay/Damage/e_DamageTypes Enum (by ref)") (InDamageDealer :type "Actor Object Reference"))
  (bind _outdamage (`/Game/Blueprints/Gameplay/Damage/bp_DamageCalculating.CalculateDamage` InDamage InDamageAdditional InDamageType InDamageTypeAdditional InDamageDealer))
  (set `self.ActualHealth` (- (`self.ActualHealth`) _outdamage)))

(event `Key|T`
  (params (Key :type "Key Structure" :default "AnyKey"))
  ;[1 1 1] School Modification
  (:`Pressed`
    (set `self.School` (`KismetMathLibrary.FClamp` (+ (`self.School`) 0.1)))))

(event `Key|Y`
  (params (Key :type "Key Structure" :default "AnyKey"))
  ;[1 1 1] School Modification
  (:`Pressed`
    (set `self.School` (`KismetMathLibrary.FClamp` (+ (`self.School`) -0.1)))))

(fn `SpawnWeaponAndSkills`
  (bind _asbp_player_controller_player (cast `/Game/Blueprints/Gameplay/Player/bp_PlayerController_Player` (`GameplayStatics.GetPlayerController` 0))
    (:`then`
      (bind _returnvalue (`|SpawnActorFromClass` (`/Game/Blueprints/Gameplay/Player/bp_PlayerController_Player.Weapon` _asbp_player_controller_player) (`KismetMathLibrary.MakeTransform` (0.0 0.0 0.0)) "AlwaysSpawn" "OverrideRootScale" null self))
      (set `self.Weapon` _returnvalue)
      (`self.K2_AttachToComponent` (`self.Weapon`) (`self.Mesh`) "RH" "KeepRelative" "KeepRelative" "KeepRelative" true)
      (for (_array_element _array_index) (`/Game/Blueprints/Gameplay/Player/bp_PlayerController_Player.RSkill` _asbp_player_controller_player)
        (bind _returnvalue_2 (`|SpawnActorFromClass` _array_element (`KismetMathLibrary.MakeTransform` (0.0 0.0 0.0)) "AlwaysSpawn" "OverrideRootScale"))
        (`KismetArrayLibrary.Array_Set` (`self.RSkill`) _array_index _returnvalue_2 true))
      (for (_array_element_2 _array_index_2) (`/Game/Blueprints/Gameplay/Player/bp_PlayerController_Player.FSkill` _asbp_player_controller_player)
        (bind _returnvalue_3 (`|SpawnActorFromClass` _array_element_2 (`KismetMathLibrary.MakeTransform` (0.0 0.0 0.0)) "AlwaysSpawn" "OverrideRootScale"))
        (`KismetArrayLibrary.Array_Set` (`self.FSkill`) _array_index_2 _returnvalue_3 true))
      (for (_array_element_3 _array_index_3) (`/Game/Blueprints/Gameplay/Player/bp_PlayerController_Player.QSkill` _asbp_player_controller_player)
        (bind _returnvalue_4 (`|SpawnActorFromClass` _array_element_3 (`KismetMathLibrary.MakeTransform` (0.0 0.0 0.0)) "AlwaysSpawn" "OverrideRootScale"))
        (`KismetArrayLibrary.Array_Set` (`self.QSkill`) _array_index_3 _returnvalue_4 true))
      (for (_array_element_4 _array_index_4) (`/Game/Blueprints/Gameplay/Player/bp_PlayerController_Player.CSkill` _asbp_player_controller_player)
        (bind _returnvalue_5 (`|SpawnActorFromClass` _array_element_4 (`KismetMathLibrary.MakeTransform` (0.0 0.0 0.0)) "AlwaysSpawn" "OverrideRootScale"))
        (`KismetArrayLibrary.Array_Set` (`self.CSkill`) _array_index_4 _returnvalue_5 true)))
    (:`CastFailed`
      _))
  (return))

(fn `UserConstructionScript`)