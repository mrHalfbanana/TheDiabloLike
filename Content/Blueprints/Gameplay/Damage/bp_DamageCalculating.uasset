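; Damage calculation Blueprint that adjusts incoming damage by the dealer's School value and returns one total.
; School is read by casting the dealer to bp_Character_Base: values below the 0.5 midpoint boost Magic and weaken Tech, values above do the reverse, and Basic is unchanged.
; Additional damage entries are scaled by their paired types and summed into the main damage.
; A failed cast returns the main damage unscaled, without the additional entries.
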(fn `CalculateDamage`
  (params (InDamage :type "Float (double-precision)") (InDamageAdditional :type "Array of Float (double-precision)") (InDamageType :type "/Game/Blueprints/Gameplay/Damage/e_DamageTypes Enum") (InDamageTypeAdditional :type "Array of /Game/Blueprints/Gameplay/Damage/e_DamageTypes Enum") (InDamageDealer :type "Actor Object Reference"))
  (returns (OutDamage :type "Float (double-precision)"))
  (locals (OutDamageBasic_LOCAL :type "Float (double-precision)") (InDamage_LOCAL :type "Float (double-precision)") (InDamageAdditional_LOCAL :type "Array of Float (double-precision)") (InDamageType_LOCAL :type "/Game/Blueprints/Gameplay/Damage/e_DamageTypes Enum") (InDamageTypeAdditional_LOCAL :type "Array of /Game/Blueprints/Gameplay/Damage/e_DamageTypes Enum") (InSchool_LOCAL :type "Float (double-precision)") (OutDamageAdditional_LOCAL :type "Array of Float (double-precision)"))
  (bind _indamageadditional_local (`local.InDamageAdditional_LOCAL`))
  (set `local.InDamage_LOCAL` InDamage)
  (set `local.InDamageAdditional_LOCAL` InDamageAdditional)
  (set `local.InDamageType_LOCAL` InDamageType)
  (set `local.InDamageTypeAdditional_LOCAL` InDamageTypeAdditional)
  (bind _asbp_character_base (cast `/Game/Blueprints/Base/bp_Character_Base` InDamageDealer)
    (:`then`
      (set `local.InSchool_LOCAL` (`/Game/Blueprints/Base/bp_Character_Base.School` _asbp_character_base))
      (switch `/Game/Blueprints/Gameplay/Damage/e_DamageTypes` (`local.InDamageType_LOCAL`)
        (:`NewEnumerator0`
          ;[0 1 0] Damage Calculating
          ;;[1 1 1] Basic Main Damage
          (set `local.OutDamageBasic_LOCAL` (`local.InDamage_LOCAL`)))
        (:`NewEnumerator1`
          ;;[1 1 1] Magic Main Damage
          (`/Engine/EditorBlueprintResources/StandardMacros.CompareFloat` (`local.InSchool_LOCAL`) 0.5
            (:`>`
              (set `local.OutDamageBasic_LOCAL` (- (`local.InDamage_LOCAL`) (* (- (`local.InSchool_LOCAL`) 0.5) (`local.InDamage_LOCAL`)))))
            (:`==`
              (set `local.OutDamageBasic_LOCAL` (`local.InDamage_LOCAL`)))
            (:`<`
              (set `local.OutDamageBasic_LOCAL` (+ (`local.InDamage_LOCAL`) (* (- 0.5 (`local.InSchool_LOCAL`)) (`local.InDamage_LOCAL`)))))))
        (:`NewEnumerator2`
          ;;[1 1 1] Tech Main Damage
          (`/Engine/EditorBlueprintResources/StandardMacros.CompareFloat` (`local.InSchool_LOCAL`) 0.5
            (:`>`
              (set `local.OutDamageBasic_LOCAL` (+ (`local.InDamage_LOCAL`) (* (- (`local.InSchool_LOCAL`) 0.5) (`local.InDamage_LOCAL`)))))
            (:`==`
              (set `local.OutDamageBasic_LOCAL` (`local.InDamage_LOCAL`)))
            (:`<`
              (set `local.OutDamageBasic_LOCAL` (- (`local.InDamage_LOCAL`) (* (- 0.5 (`local.InSchool_LOCAL`)) (`local.InDamage_LOCAL`))))))))
      ;[0 0 1] Additional
      (if (> (`KismetArrayLibrary.Array_Length` _indamageadditional_local) 0)
        (for (_array_element _array_index) _indamageadditional_local
          (switch `/Game/Blueprints/Gameplay/Damage/e_DamageTypes` (`|GetArrayItem` (`local.InDamageTypeAdditional_LOCAL`) _array_index)
            (:`NewEnumerator0`
              ;;[0 1 0] Damage Calculating
              ;;;[1 1 1] Basic Main Damage
              (`KismetArrayLibrary.Array_Set` (`local.OutDamageAdditional_LOCAL`) _array_index _array_element true))
            (:`NewEnumerator1`
              ;;;[1 1 1] Magic Main Damage
              (`/Engine/EditorBlueprintResources/StandardMacros.CompareFloat` (`local.InSchool_LOCAL`) 0.5
                (:`>`
                  (`KismetArrayLibrary.Array_Set` (`local.OutDamageAdditional_LOCAL`) _array_index (- _array_element (* (- (`local.InSchool_LOCAL`) 0.5) _array_element)) true))
                (:`==`
                  (`KismetArrayLibrary.Array_Set` (`local.OutDamageAdditional_LOCAL`) _array_index _array_element true))
                (:`<`
                  (`KismetArrayLibrary.Array_Set` (`local.OutDamageAdditional_LOCAL`) _array_index (+ _array_element (* (- 0.5 (`local.InSchool_LOCAL`)) _array_element)) true))))
            (:`NewEnumerator2`
              ;;;[1 1 1] Tech Main Damage
              (`/Engine/EditorBlueprintResources/StandardMacros.CompareFloat` (`local.InSchool_LOCAL`) 0.5
                (:`>`
                  (`KismetArrayLibrary.Array_Set` (`local.OutDamageAdditional_LOCAL`) _array_index (+ _array_element (* (- (`local.InSchool_LOCAL`) 0.5) _array_element)) true))
                (:`==`
                  (`KismetArrayLibrary.Array_Set` (`local.OutDamageAdditional_LOCAL`) _array_index _array_element true))
                (:`<`
                  (`KismetArrayLibrary.Array_Set` (`local.OutDamageAdditional_LOCAL`) _array_index (- _array_element (* (- 0.5 (`local.InSchool_LOCAL`)) _array_element)) true))))))
        ;[0 1 1] Out
        (for _array_element_2 (`local.OutDamageAdditional_LOCAL`) :!label _label
          (set `local.OutDamageBasic_LOCAL` (+ _array_element_2 (`local.OutDamageBasic_LOCAL`))))))
    (:`CastFailed`
      ;[1 1 1] Basic Main Damage
      (set `local.OutDamageBasic_LOCAL` (`local.InDamage_LOCAL`))
      (goto _label)))
  (return (`local.OutDamageBasic_LOCAL`)))