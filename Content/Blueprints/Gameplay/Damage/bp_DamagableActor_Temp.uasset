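; Temporary damageable actor that holds a Health value, shows it on a text render and is destroyed when it runs out.
; DoDamage passes primary and additional damage amounts and types, plus the dealer, to CalculateDamage and subtracts the result from Health.
; Tick refreshes the health text every frame.
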(event `self.ReceiveTick`
  (params (DeltaSeconds :type "Float (single-precision)"))
  (`TextRenderComponent.K2_SetText` (`self.TextRender`) (`KismetTextLibrary.Conv_DoubleToText` (`self.Health`) "HalfToEven")))

(event `/Game/Blueprints/Gameplay/Damage/i_Damagable.DoDamage`
  (params (InDamage :type "Float (single-precision)") (InDamageAdditional :type "Array of Float (single-precision) (by ref)") (InDamageType :type "/Game/Blueprints/Gameplay/Damage/e_DamageTypes Enum") (InDamageTypeAdditional :type "Array of /Game/Blueprints/Gameplay/Damage/e_DamageTypes Enum (by ref)") (InDamageDealer :type "Actor Object Reference"))
  (bind _outdamage (`/Game/Blueprints/Gameplay/Damage/bp_DamageCalculating.CalculateDamage` InDamage InDamageAdditional InDamageType InDamageTypeAdditional InDamageDealer))
  (bind _output_get (set `self.Health` (- (`self.Health`) _outdamage)))
  (if (<= _output_get 0.0)
    (`self.K2_DestroyActor`)))

(fn `UserConstructionScript`)