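; Gameplay game mode that spawns and possesses the player character when a player logs in, in a flow marked temporary.
; PostLogin stores the first player start's transform as the controller's last checkpoint, then after fixed delays spawns the pawn and flags the level as generated.
; SpawnPawn replaces any existing pawn at that checkpoint, sets health and armor to GameInstance maximums, and applies the selected class via SwitchSpec.
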(event `self.ReceiveBeginPlay`
  ;[0 1 0] Game Instance Reference
  (bind _asbp_game_instance (cast `/Game/Blueprints/Base/bp_GameInstance` (`GameplayStatics.GetGameInstance`)))
  (set `self.GameInstanceRef` _asbp_game_instance))

(event `self.K2_PostLogin`
  (params (NewPlayer :type "PlayerController Object Reference"))
  ;[1 1 0] Player Spawn (TEMP)
  (bind _asbp_player_controller_player (cast `/Game/Blueprints/Gameplay/Player/bp_PlayerController_Player` NewPlayer))
  (bind _output_get (set `self.PlayerControllerRef` _asbp_player_controller_player))
  (`self.FindPlayerStartOnLevel`)
  (`KismetSystemLibrary.Delay` 1.0)
  (`self.SpawnPawn` _output_get)
  (`KismetSystemLibrary.Delay` 1.0)
  (set `self.LevelGenerated?` true))

(fn `FindPlayerStartOnLevel`
  (bind _outactors (`GameplayStatics.GetAllActorsOfClass` "/Game/Blueprints/Base/bp_PlayerStart_Base.bp_PlayerStart_Base_C"))
  (bind _output (`|GetArrayItem` _outactors))
  (`/Engine/EditorBlueprintResources/StandardMacros.IsValid` _output
    (:`Is Valid`
      (set `/Game/Blueprints/Gameplay/Player/bp_PlayerController_Player.LastCheckpoint` (`self.GetTransform` _output) (`self.PlayerControllerRef`))
      (return))))

(fn `SpawnPawn`
  (params (InController :type "Controller Object Reference"))
  (bind _returnvalue (`Controller.K2_GetPawn` InController))
  (bind _playercontrollerref (`self.PlayerControllerRef`))
  (bind ((`HealthMax_14_AD75400E4E740F2317A1C298B8CF5828` _healthmax) (`ArmorMax_18_CB46BE734139D6EAC84335B5C10D9C5D` _armormax)) (break `/Game/Blueprints/Gameplay/Player/Enums_and_Structs/str_PlayerInfo` (`/Game/Blueprints/Base/bp_GameInstance.PlayerInfo` (`self.GameInstanceRef`))))
  (`/Engine/EditorBlueprintResources/StandardMacros.IsValid` _returnvalue
    (:`Is Valid`
      (`self.K2_DestroyActor` _returnvalue))
    (:`Is Not Valid`
      _))
  (bind _returnvalue_2 (`|SpawnActorFromClass` "/Game/Blueprints/Gameplay/Player/bp_Character_Player.bp_Character_Player_C" (`/Game/Blueprints/Gameplay/Player/bp_PlayerController_Player.LastCheckpoint` (`self.PlayerControllerRef`)) "AlwaysSpawn" "OverrideRootScale" null _healthmax _armormax))
  (set `self.PlayerPawnRef` _returnvalue_2)
  (`Controller.Possess` _playercontrollerref (`self.PlayerPawnRef`))
  (set `/Game/Blueprints/Gameplay/Player/bp_PlayerController_Player.PlayerPawnRef` (`self.PlayerPawnRef`) _playercontrollerref)
  (set `/Game/Blueprints/Gameplay/Player/bp_PlayerController_Player.SelectedClass` (`.SelectedClass_2_445486E14F13D3497E66449AB794AF65` (break `/Game/Blueprints/Gameplay/Player/Enums_and_Structs/str_PlayerInfo` (`/Game/Blueprints/Base/bp_GameInstance.PlayerInfo` (`self.GameInstanceRef`)))) _playercontrollerref)
  (set `/Game/Blueprints/Gameplay/Player/bp_PlayerController_Player.ActiveSpec` 0 _playercontrollerref)
  (`/Game/Blueprints/Gameplay/Player/bp_PlayerController_Player.SwitchSpec` _playercontrollerref)
  (return))

(fn `UserConstructionScript`
  (`parent.UserConstructionScript`))