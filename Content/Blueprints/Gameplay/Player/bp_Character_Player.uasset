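; Player character Blueprint with a top camera and a side camera.
; A temporary Z key binding toggles the active state of both cameras.
; The Death event forwards to the player controller's Death when the controller is a bp_PlayerController_Player.
; ActualSpecSets applies a given material to the mesh's first slot, and the construction script only calls the parent's.
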(event `Key|Z`
  (params (Key :type "Key Structure" :default "AnyKey"))
  ;[1 1 0] Toggle Cameras (TEMP)
  (:`Pressed`
    (`ActorComponent.ToggleActive` (`self.TopCamera`))
    (`ActorComponent.ToggleActive` (`self.SideCamera`))))

(event `self.Death`
  ;[1 1 1] Death
  (bind _asbp_player_controller_player (cast `/Game/Blueprints/Gameplay/Player/bp_PlayerController_Player` (`self.GetController`)))
  (`/Game/Blueprints/Gameplay/Player/bp_PlayerController_Player.Death` _asbp_player_controller_player))

(fn `ActualSpecSets`
  (params (InMaterial :type "Material Object Reference"))
  (`PrimitiveComponent.SetMaterial` (`self.Mesh`) 0 InMaterial))

(fn `UserConstructionScript`
  (`parent.UserConstructionScript`))