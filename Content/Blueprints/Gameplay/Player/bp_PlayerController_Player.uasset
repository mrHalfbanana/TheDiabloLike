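; Player controller for top-down style gameplay, handling world-axis movement, cursor-facing rotation and switching between two specs.
; On BeginPlay it caches GameInstance and GameMode, sets game-only input and shows an error manager widget.
; Movement axes yaw the pawn toward an object trace under the cursor, logging invalid-pawn errors to the GameInstance.
; Spec switching passes class materials to the pawn, while attack, skill and death events only print placeholders.
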(event `self.ReceiveBeginPlay`
  ;[0 1 0] Get All References
  (`self.GetAllReferences`)
  ;[0 1 0] Set Focus to Game
  (`WidgetBlueprintLibrary.SetInputMode_GameOnly` self)
  ;[0 1 0] Show Error Manager
  (`self.ShowErrorManager`))

(event `InputAxis|MoveForward`
  (params (AxisValue :type "Float (single-precision)"))
  (bind _returnvalue (`self.K2_GetPawn`))
  ;[0 1 0] Movement
  (`/Engine/EditorBlueprintResources/StandardMacros.IsValid` _returnvalue
    (:`Is Valid`
      (`Pawn.AddMovementInput` _returnvalue (1.0 0.0 0.0) AxisValue false)
      (`self.RotateToFaceCursor` :!label _label))
    (:`Is Not Valid`
      ;;[1 1 1] Error Handling
      (`/Game/Blueprints/Base/bp_GameInstance.SaveErrors` (`self.GameInstanceRef`) (make `/Game/Blueprints/ErrorandDebugging/str_ErrorStruct` (`KismetMathLibrary.Now`) "Controlled Pawn Not Valid (Movement)" self) :!label _label_2))))

(event `InputAxis|MoveRight`
  (params (AxisValue :type "Float (single-precision)"))
  (bind _returnvalue (`self.K2_GetPawn`))
  ;[0 1 0] Movement
  (`/Engine/EditorBlueprintResources/StandardMacros.IsValid` _returnvalue
    (:`Is Valid`
      (`Pawn.AddMovementInput` _returnvalue (0.0 1.0 0.0) AxisValue false)
      (goto _label))
    (:`Is Not Valid`
      (goto _label_2))))

(event `SaveLastCheckPoint`)

(event `InputAction|QuitGameBtn`
  (params (Key :type "Key Structure" :default "AnyKey"))
  ;[0 1 0] Quit Game
  (:`Pressed`
    (`KismetSystemLibrary.QuitGame` null "Quit")))

(event `ShowErrorManager`
  ;[0 1 0] Show Error Manager
  (bind _returnvalue (`|CreateWidget` "/Game/Blueprints/ErrorandDebugging/w_ErrorManagerUI.w_ErrorManagerUI_C"))
  (set `self.ErrorManagerRef` _returnvalue)
  (`UserWidget.AddToViewport` (`self.ErrorManagerRef`) 0))

(event `TempErrorAdd`
  ;[0 0 1] JUST FOR EXAMPLE!
  (bind _asbp_game_instance (cast `/Game/Blueprints/Base/bp_GameInstance` (`GameplayStatics.GetGameInstance`)))
  (`/Game/Blueprints/Base/bp_GameInstance.SaveErrors` _asbp_game_instance (make `/Game/Blueprints/ErrorandDebugging/str_ErrorStruct` (`KismetMathLibrary.GetDate` (`KismetMathLibrary.Now`)) "Error Message" self)))

(event `InputAction|LMB`
  (params (Key :type "Key Structure" :default "AnyKey"))
  (:`Pressed`
    (`KismetSystemLibrary.PrintString` "LMB")))

(event `InputAction|QSkill`
  (params (Key :type "Key Structure" :default "AnyKey"))
  (:`Pressed`
    (`KismetSystemLibrary.PrintString` "Q Skill")))

(event `InputAction|RSkill`
  (params (Key :type "Key Structure" :default "AnyKey"))
  (:`Pressed`
    (`KismetSystemLibrary.PrintString` "R Skill")))

(event `InputAction|FSkill`
  (params (Key :type "Key Structure" :default "AnyKey"))
  (:`Pressed`
    (`KismetSystemLibrary.PrintString` "F Skill")))

(event `InputAction|CSkill`
  (params (Key :type "Key Structure" :default "AnyKey"))
  (:`Pressed`
    (`KismetSystemLibrary.PrintString` "C Skill")))

(event `InputAction|SpecSwitch`
  (params (Key :type "Key Structure" :default "AnyKey"))
  (:`Pressed`
    (`self.SwitchSpec`)))

(event `Death`
  (`KismetSystemLibrary.PrintString` "Death"))

(fn `CalculateSchool`
  (set `/Game/Blueprints/Gameplay/Player/bp_Character_Player.School` 0.0 (`self.PlayerPawnRef`)))

(fn `GetAllReferences`
  (bind _asbp_game_instance (cast `/Game/Blueprints/Base/bp_GameInstance` (`GameplayStatics.GetGameInstance`))
    (:`then`
      (set `self.GameInstanceRef` _asbp_game_instance))
    (:`CastFailed`
      _))
  (bind _asbp_game_mode_game_play (cast `/Game/Blueprints/Gameplay/bp_GameMode_GamePlay` (`GameplayStatics.GetGameMode`))
    (:`then`
      (set `self.GameModeRef` _asbp_game_mode_game_play))
    (:`CastFailed`
      _))
  (return))

(fn `RotateToFaceCursor`
  (bind _returnvalue (`self.K2_GetPawn`))
  (bind (_returnvalue_roll _returnvalue_pitch) (`KismetMathLibrary.BreakRotator` (`self.K2_GetActorRotation` _returnvalue)))
  (bind (_returnvalue_roll_2 _returnvalue_pitch_2 _returnvalue_yaw) (`KismetMathLibrary.BreakRotator` (`KismetMathLibrary.FindLookAtRotation` (`self.K2_GetActorLocation` _returnvalue) (`.Location` (`GameplayStatics.BreakHitResult` (`self.GetHitResultUnderCursorForObjects` (`|MakeArray` "ObjectTypeQuery7" :!type "EObjectTypeQuery Enum")))))))
  (`self.K2_SetActorRotation` _returnvalue (`KismetMathLibrary.MakeRotator` _returnvalue_roll _returnvalue_pitch _returnvalue_yaw) false))

(fn `SwitchSpec`
  (bind ((`ClassMaterials_TEMP_7_F1016EB44E28A72CD5E594871E113BF3` _classmaterials_temp)) (break `/Game/Blueprints/Gameplay/Player/Enums_and_Structs/str_PlayerInfo` (`/Game/Blueprints/Base/bp_GameInstance.PlayerInfo` (`self.GameInstanceRef`))))
  (switch `int` (`self.ActiveSpec`)
    (:`0`
      (bind _output_get (set `self.ActiveSpec` 1))
      (`/Game/Blueprints/Gameplay/Player/bp_Character_Player.ActualSpecSets` (`self.PlayerPawnRef`) (`|GetArrayItem` _classmaterials_temp _output_get)))
    (:`1`
      (bind _output_get_2 (set `self.ActiveSpec` 0))
      (`/Game/Blueprints/Gameplay/Player/bp_Character_Player.ActualSpecSets` (`self.PlayerPawnRef`) (`|GetArrayItem` _classmaterials_temp _output_get_2)))))

(fn `UserConstructionScript`
  (`parent.UserConstructionScript`))