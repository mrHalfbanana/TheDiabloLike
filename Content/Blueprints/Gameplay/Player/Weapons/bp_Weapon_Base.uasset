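; Base weapon Blueprint for the player that provides a hitscan Fire event aimed at the mouse cursor.
; Fire line-traces on the Visibility channel from the weapon's location to the world point under the cursor.
; A hit actor implementing I_Damagable receives DoDamageMessage with main and additional damage, their types, and PawnRef as dealer.
; Debug output remains in place: a "PEW PEW" print and timed trace drawing.
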(event `Fire`
  (`KismetSystemLibrary.PrintString` "PEW PEW")
  (bind (_outhit _returnvalue) (`KismetSystemLibrary.LineTraceSingle` :`Start` (`self.K2_GetActorLocation`) :`End` (`.Location` (`GameplayStatics.BreakHitResult` (`PlayerController.GetHitResultUnderCursorByChannel` (`GameplayStatics.GetPlayerController` 0) "TraceTypeQuery1" true))) :`TraceChannel` "TraceTypeQuery1" :`DrawDebugType` "ForDuration"))
  (if (and _returnvalue (`KismetSystemLibrary.DoesImplementInterface` (`.HitActor` (`GameplayStatics.BreakHitResult` _outhit)) "/Game/Blueprints/Gameplay/Damage/i_Damagable.i_Damagable_C"))
    (message `/Game/Blueprints/Gameplay/Damage/i_Damagable.DoDamage` (`.HitActor` (`GameplayStatics.BreakHitResult` _outhit)) (`self.DamageMain`) (`self.DamageAdditional`) (`self.DamageTypeMain`) (`self.DamageTypeAdditional`) (`self.PawnRef`))))

(fn `UserConstructionScript`)