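; Player controller for the main menu that manages which UI screen is on screen.
; On BeginPlay it shows the main menu and sets UI-only input mode without locking the mouse.
; Events show the main menu and class selection widgets, creating each once with a controller reference and caching it for reuse.
; A separate event removes whichever widget is passed in from its parent.
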(event `self.ReceiveBeginPlay`
  ;[1 1 1] BEGIN PLAY EVENT
  ;;[0 1 0] First Load of Main Menu
  (`self.ShowMainMenu`)
  ;;[0 1 0] Focus Cursor to UI Only
  (`WidgetBlueprintLibrary.SetInputMode_UIOnlyEx` self))

(event `ShowMainMenu`
  ;[0 1 0] MainMenu
  (`/Engine/EditorBlueprintResources/StandardMacros.IsValid` (`self.MainMenuWidget`)
    (:`Is Valid`
      _)
    (:`Is Not Valid`
      (bind _returnvalue (`|CreateWidget` "/Game/Blueprints/MainMenu/Widgets/w_MainMenu.w_MainMenu_C" null self))
      (set `self.MainMenuWidget` _returnvalue)))
  (`UserWidget.AddToViewport` (`self.MainMenuWidget`) 0))

(event `ShowClassSelectionMenu`
  ;[0 1 0] Class Selection
  (`/Engine/EditorBlueprintResources/StandardMacros.IsValid` (`self.ClassSelectionWidget`)
    (:`Is Valid`
      _)
    (:`Is Not Valid`
      (bind _returnvalue (`|CreateWidget` "/Game/Blueprints/MainMenu/Widgets/w_ClassSelection.w_ClassSelection_C" null self))
      (set `self.ClassSelectionWidget` _returnvalue)))
  (`UserWidget.AddToViewport` (`self.ClassSelectionWidget`) 0))

(event `RemovePrevWidgets`
  (params (InWidgetToRemove :type "Widget Object Reference"))
  ;[0 1 0] Remove Previous Widgets
  (`Widget.RemoveFromParent` InWidgetToRemove))

(fn `UserConstructionScript`
  (`parent.UserConstructionScript`))